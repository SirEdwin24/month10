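; BP_Container is a puzzle container actor that counts objects entering its trigger and reports completion to the puzzle manager.
; On BeginPlay it caches a reference to BP_PuzzleManager.
; Each trigger overlap runs through a one-second delay, then increments the count with no actor filtering.
; When the count equals the maximum, it clamps the manager's solved-puzzle count to its range, then adds one.
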(event `self.ReceiveBeginPlay`
  (bind _returnvalue (`GameplayStatics.GetActorOfClass` "/Game/BP_Actors/BP_PuzzleManager.BP_PuzzleManager_C"))
  (set `self.PuzzleRef` _returnvalue))

(event `self.Trigger.OnComponentBeginOverlap`
  (params (OverlappedComponent :type "PrimitiveComponent Object Reference") (OtherActor :type "Actor Object Reference") (OtherComp :type "PrimitiveComponent Object Reference") (OtherBodyIndex :type Integer) (bFromSweep :type Boolean) (SweepResult :type "HitResult Structure (by ref)"))
  (bind _puzzleref (`self.PuzzleRef`))
  ;[1 1 1] Count number of object in container and add 1 to cur puzzlee to check if puzzle complete
  (`KismetSystemLibrary.Delay` 1.0)
  (set `self.CurCount` (+ (`self.CurCount`) 1))
  (if (== (`self.CurCount`) (`self.MaxCount`))
    (set `/Game/BP_Actors/BP_PuzzleManager.CurPuzzles` (+ (`KismetMathLibrary.Clamp` (`/Game/BP_Actors/BP_PuzzleManager.CurPuzzles` _puzzleref) 0 (`/Game/BP_Actors/BP_PuzzleManager.MaxPuzzles` _puzzleref)) 1) _puzzleref)))

(fn `UserConstructionScript`)